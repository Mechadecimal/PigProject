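; Automatic sliding double door that opens for BP_Pig and can reorient that pig's camera as it leaves.
; Box overlaps play or reverse a timeline that slides LDoor and RDoor apart in mirrored motion, with a beep on each trigger.
; When ShouldRotateCamera is set, end overlap uses a dot product against the Arrow's forward vector to snap the pig's SpringArm to FrontRot or BackRot, depending on the exit side.
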(event `OpenDoor`
  (bind (_direction _newtrack_0) (`Timeline|Timeline_0` :!label _label)
    (:`Update`
      (bind _returnvalue (`KismetMathLibrary.VLerp` (0.0 0.0 0.0) (0.0 65.0 0.0) _newtrack_0))
      (`SceneComponent.K2_SetRelativeLocation` (`self.LDoor`) _returnvalue false false)
      (`SceneComponent.K2_SetRelativeLocation` (`self.RDoor`) (`KismetMathLibrary.NegateVector` _returnvalue) false false))))

(event `CloseDoor`
  (goto _label :!via `Reverse`))

(event `self.Box.OnComponentBeginOverlap`
  (params (OverlappedComponent :type "PrimitiveComponent Object Reference") (OtherActor :type "Actor Object Reference") (OtherComp :type "PrimitiveComponent Object Reference") (OtherBodyIndex :type Integer) (bFromSweep :type Boolean) (SweepResult :type "HitResult Structure (by ref)"))
  (if (== (`GameplayStatics.GetObjectClass` OtherActor) "/Game/LevelPrototyping/Blueprints/BP_Pig.BP_Pig_C")
    (`self.OpenDoor`)
    (`GameplayStatics.PlaySoundAtLocation` "/Game/Sounds/ComputerBeeps.ComputerBeeps" (`self.K2_GetActorLocation`) (struct) 1.0 1.0 0.0 null null null null)))

(event `self.Box.OnComponentEndOverlap`
  (params (OverlappedComponent :type "PrimitiveComponent Object Reference") (OtherActor :type "Actor Object Reference") (OtherComp :type "PrimitiveComponent Object Reference") (OtherBodyIndex :type Integer))
  (bind _arrow (`self.Arrow`))
  (if (== (`GameplayStatics.GetObjectClass` OtherActor) "/Game/LevelPrototyping/Blueprints/BP_Pig.BP_Pig_C")
    (`self.CloseDoor`)
    (`GameplayStatics.PlaySoundAtLocation` "/Game/Sounds/ComputerBeeps.ComputerBeeps" (`self.K2_GetActorLocation`) (struct) 1.0 1.0 0.0 null null null null)
    (if (`self.ShouldRotateCamera`)
      (bind _asbp_pig (cast `/Game/LevelPrototyping/Blueprints/BP_Pig` OtherActor))
      (`SceneComponent.K2_SetWorldRotation` (`/Game/LevelPrototyping/Blueprints/BP_Pig.SpringArm` _asbp_pig) (`KismetMathLibrary.SelectRotator` (`self.FrontRot`) (`self.BackRot`) (>= (`KismetMathLibrary.Dot_VectorVector` (`SceneComponent.GetForwardVector` _arrow) (`KismetMathLibrary.GetDirectionUnitVector` (`SceneComponent.K2_GetComponentLocation` _arrow) (`self.K2_GetActorLocation` OtherActor))) 0.0)) false true))))

(fn `UserConstructionScript`)