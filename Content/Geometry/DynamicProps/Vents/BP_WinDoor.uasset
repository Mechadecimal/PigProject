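; BP_WinDoor is a door that ends the game once a BP_Pig passes through it.
; A box overlap opens the door when the pig enters and closes it when the pig leaves, playing computer beeps each time.
; On exit, a dot product against the Arrow's forward vector checks the pig's side.
; A pig behind the arrow triggers Endgame on BP_TopDownGameMode.
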(event `self.Box.OnComponentBeginOverlap`
  (params (OverlappedComponent :type "PrimitiveComponent Object Reference") (OtherActor :type "Actor Object Reference") (OtherComp :type "PrimitiveComponent Object Reference") (OtherBodyIndex :type Integer) (bFromSweep :type Boolean) (SweepResult :type "HitResult Structure (by ref)"))
  (if (== (`GameplayStatics.GetObjectClass` OtherActor) "/Game/LevelPrototyping/Blueprints/BP_Pig.BP_Pig_C")
    (`self.OpenDoor`)
    (`GameplayStatics.PlaySoundAtLocation` "/Game/Sounds/ComputerBeeps.ComputerBeeps" (`self.K2_GetActorLocation`) (struct) 1.0 1.0 0.0 null null null null)))

(event `self.Box.OnComponentEndOverlap`
  (params (OverlappedComponent :type "PrimitiveComponent Object Reference") (OtherActor :type "Actor Object Reference") (OtherComp :type "PrimitiveComponent Object Reference") (OtherBodyIndex :type Integer))
  (bind _arrow (`self.Arrow`))
  (if (== (`GameplayStatics.GetObjectClass` OtherActor) "/Game/LevelPrototyping/Blueprints/BP_Pig.BP_Pig_C")
    (`self.CloseDoor`)
    (`GameplayStatics.PlaySoundAtLocation` "/Game/Sounds/ComputerBeeps.ComputerBeeps" (`self.K2_GetActorLocation`) (struct) 1.0 1.0 0.0 null null null null)
    (if (== (>= (`KismetMathLibrary.Dot_VectorVector` (`SceneComponent.GetForwardVector` _arrow) (`KismetMathLibrary.GetDirectionUnitVector` (`SceneComponent.K2_GetComponentLocation` _arrow) (`self.K2_GetActorLocation` OtherActor))) 0.0) false)
      (`self.EndGame`))))

(event `EndGame`
  (bind _asbp_top_down_game_mode (cast `/Game/LevelPrototyping/Blueprints/BP_TopDownGameMode` (`GameplayStatics.GetGameMode`)))
  (`/Game/LevelPrototyping/Blueprints/BP_TopDownGameMode.Endgame` _asbp_top_down_game_mode))

(fn `UserConstructionScript`
  (`parent.UserConstructionScript`))