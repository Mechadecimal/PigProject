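; BP_Prop_Vent is a warp vent that teleports BP_Pig to the partner vent sharing its WarpID, found on BeginPlay.
; Trigger overlap warps immediately in one PigMoveState, otherwise binds entry to the pig's dash dispatcher until overlap ends.
; Entry stuns, hides and freezes the pig, moves it beyond the partner's ExitDirection and optionally re-aims the camera.
; After short delays, the partner's exit event restores visibility, gravity, collision and control.
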(event `self.ReceiveBeginPlay`
  (bind _outactors (`GameplayStatics.GetAllActorsOfClass` "BP_Prop_Vent_C"))
  (for _array_element _outactors
    (if (and (== (`/Game/Geometry/DynamicProps/Vents/BP_Prop_Vent.warpID` _array_element) (`self.warpID`)) (!= _array_element self))
      (set `self.PartnerRef` _array_element)
      (break))))

(event `enterEvent`
  (params (pig :type "/Game/LevelPrototyping/Blueprints/BP_Pig Object Reference"))
  (bind _partnerref (`self.PartnerRef`))
  (bind _exitdirection (`/Game/Geometry/DynamicProps/Vents/BP_Prop_Vent.exitDirection` (`self.PartnerRef`)))
  (bind (_returnvalue_roll _returnvalue_pitch _returnvalue_yaw) (`KismetMathLibrary.BreakRotator` (`SceneComponent.K2_GetComponentRotation` (`Actor.RootComponent` _partnerref))))
  (`/Engine/EditorBlueprintResources/StandardMacros.IsValid` (`self.PartnerRef`)
    (:`Is Valid`
      (`/Game/LevelPrototyping/Blueprints/BP_Pig.pigStun` pig)
      (set `CharacterMovementComponent.GravityScale` 0.0 (`Character.CharacterMovement` pig))
      (`PrimitiveComponent.SetCollisionEnabled` (`Character.CapsuleComponent` pig) "NoCollision")
      (`SceneComponent.SetVisibility` (`Character.Mesh` pig) false false)
      (set `MovementComponent.Velocity` (0.0 0.0 0.0) (`Character.CharacterMovement` pig))
      (set `self.pigTempLocation` (`self.K2_GetActorLocation` pig))
      (bind _output_get (set `self.pigTempCamRotation` (`SceneComponent.K2_GetComponentRotation` (`/Game/LevelPrototyping/Blueprints/BP_Pig.SpringArm` pig))))
      (set `self.FinalCam` (`KismetMathLibrary.MakeRotator` (.roll _output_get) (.pitch _output_get) (+ (+ _returnvalue_yaw 180.0) (`/Game/Geometry/DynamicProps/Vents/BP_Prop_Vent.cameraDegreeBump` _partnerref))))
      (`KismetSystemLibrary.Delay` 0.25)
      (`self.K2_TeleportTo` pig (+ (`SceneComponent.K2_GetComponentLocation` _exitdirection) (* (`SceneComponent.GetForwardVector` _exitdirection) 500)) (`self.K2_GetActorRotation` pig))
      (if (`self.adjustCameraRotation`)
        (`SceneComponent.K2_SetWorldRotation` (`/Game/LevelPrototyping/Blueprints/BP_Pig.SpringArm` pig) (`self.FinalCam`) false true))
      (set `MovementComponent.Velocity` (0.0 0.0 0.0) (`Character.CharacterMovement` pig))
      (`KismetSystemLibrary.Delay` 0.75)
      (`self.exitEvent` (`self.PartnerRef`) pig))))

(event `exitEvent`
  (params (pig :type "/Game/LevelPrototyping/Blueprints/BP_Pig Object Reference"))
  (bind _charactermovement (`Character.CharacterMovement` pig))
  (set `MovementComponent.Velocity` (0.0 0.0 0.0) _charactermovement)
  (`SceneComponent.SetVisibility` (`Character.Mesh` pig) true false)
  (`KismetSystemLibrary.Delay` 0.25)
  (set `CharacterMovementComponent.GravityScale` 1.5 _charactermovement)
  (`PrimitiveComponent.SetCollisionEnabled` (`Character.CapsuleComponent` pig) "QueryAndPhysics")
  (`/Game/LevelPrototyping/Blueprints/BP_Pig.pigUnstun` pig)
  (set `/Game/LevelPrototyping/Blueprints/BP_Pig.pigMoveState` "NewEnumerator0" pig))

(event `self.warpTrigger.OnComponentBeginOverlap`
  (params (OverlappedComponent :type "PrimitiveComponent Object Reference") (OtherActor :type "Actor Object Reference") (OtherComp :type "PrimitiveComponent Object Reference") (OtherBodyIndex :type Integer) (bFromSweep :type Boolean) (SweepResult :type "HitResult Structure (by ref)"))
  (if (== (`GameplayStatics.GetObjectClass` OtherActor) "/Game/LevelPrototyping/Blueprints/BP_Pig.BP_Pig_C")
    (bind _asbp_pig (cast `/Game/LevelPrototyping/Blueprints/BP_Pig` OtherActor))
    (if (`|EnumEquality` (`/Game/LevelPrototyping/Blueprints/BP_Pig.pigMoveState` _asbp_pig) "NewEnumerator0")
      (`self.enterEvent` _asbp_pig)
      (else
        (add `/Game/LevelPrototyping/Blueprints/BP_Pig.dashDispatcher` _asbp_pig (delegate `CustomEvent_0`))))))

(event `CustomEvent_0`
  (`self.enterEvent` (stale `self.warpTrigger.OnComponentBeginOverlap` _asbp_pig)))

(event `self.warpTrigger.OnComponentEndOverlap`
  (params (OverlappedComponent :type "PrimitiveComponent Object Reference") (OtherActor :type "Actor Object Reference") (OtherComp :type "PrimitiveComponent Object Reference") (OtherBodyIndex :type Integer))
  (if (== (`GameplayStatics.GetObjectClass` OtherActor) "/Game/LevelPrototyping/Blueprints/BP_Pig.BP_Pig_C")
    (bind _asbp_pig (cast `/Game/LevelPrototyping/Blueprints/BP_Pig` OtherActor))
    (remove `/Game/LevelPrototyping/Blueprints/BP_Pig.dashDispatcher` _asbp_pig (delegate `CustomEvent_0`))))

(fn `UserConstructionScript`)