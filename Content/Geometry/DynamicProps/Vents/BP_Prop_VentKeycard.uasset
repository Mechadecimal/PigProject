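; A keycard-locked vent prop that BP_Pig can enter through a warp trigger once it is unlocked.
; On overlap, a locked vent searches the pig's keycards, consumes the one matching KeycardID, activates and plays beeps.
; An active vent calls EnterEvent if the pig is in a specific move state, otherwise binds to its dash dispatcher to enter on dash.
; Leaving the trigger unbinds that dash event.
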(event `unlockEvent`
  (set `self.isActive` true)
  (`GameplayStatics.PlaySoundAtLocation` "/Game/Sounds/ComputerBeeps.ComputerBeeps" (`self.K2_GetActorLocation`) (struct) 1.0 1.0 0.0 null null null null))

(event `self.warpTrigger.OnComponentBeginOverlap`
  (params (OverlappedComponent :type "PrimitiveComponent Object Reference") (OtherActor :type "Actor Object Reference") (OtherComp :type "PrimitiveComponent Object Reference") (OtherBodyIndex :type Integer) (bFromSweep :type Boolean) (SweepResult :type "HitResult Structure (by ref)"))
  (if (== (`GameplayStatics.GetObjectClass` OtherActor) "/Game/LevelPrototyping/Blueprints/BP_Pig.BP_Pig_C")
    (bind _asbp_pig (cast `/Game/LevelPrototyping/Blueprints/BP_Pig` OtherActor))
    (if (`self.IsActive`)
      (if (`|EnumEquality` (`/Game/LevelPrototyping/Blueprints/BP_Pig.pigMoveState` _asbp_pig) "NewEnumerator2")
        (`self.enterEvent` _asbp_pig)
        (else
          (add `/Game/LevelPrototyping/Blueprints/BP_Pig.dashDispatcher` _asbp_pig (delegate `CustomEvent`) :!label _label)))
      (else
        (bind _unlocked (`self.tryUnlock` _asbp_pig))
        (if _unlocked
          (`self.unlockEvent`)
          (goto _label))))))

(event `CustomEvent`
  (if (`self.IsActive`)
    (`self.enterEvent` (stale `self.warpTrigger.OnComponentBeginOverlap` _asbp_pig))))

(event `self.warpTrigger.OnComponentEndOverlap`
  (params (OverlappedComponent :type "PrimitiveComponent Object Reference") (OtherActor :type "Actor Object Reference") (OtherComp :type "PrimitiveComponent Object Reference") (OtherBodyIndex :type Integer))
  (if (== (`GameplayStatics.GetObjectClass` OtherActor) "/Game/LevelPrototyping/Blueprints/BP_Pig.BP_Pig_C")
    (bind _asbp_pig (cast `/Game/LevelPrototyping/Blueprints/BP_Pig` OtherActor))
    (remove `/Game/LevelPrototyping/Blueprints/BP_Pig.dashDispatcher` _asbp_pig (delegate `CustomEvent`))))

(fn `tryUnlock`
  (params (pig :type "/Game/LevelPrototyping/Blueprints/BP_Pig Object Reference"))
  (returns (unlocked :type Boolean))
  (bind _keycards (`/Game/LevelPrototyping/Blueprints/BP_Pig.keycards` pig))
  (for (_array_element _array_index) _keycards
    (if (== _array_element (`self.keycardID`))
      (`KismetArrayLibrary.Array_Remove` _keycards _array_index)
      (set `self.IsActive` true)
      (break)))
  (return (`self.IsActive`)))

(fn `UserConstructionScript`
  (`parent.UserConstructionScript`))