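; BP_Prop_Dynamic is a physical prop that can bounce or break when BP_TopDownCharacter hits its cube, optionally only in one pig move state (PigDashNeeded).
; If bouncy, it launches the character away from its center and replays a scale timeline on the cube.
; If destructible and not fragile, it enables gravity on the cube, waits, then shrinks it with a timeline and destroys the actor.
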(event `self.Cube.OnComponentHit`
  (params (HitComponent :type "PrimitiveComponent Object Reference") (OtherActor :type "Actor Object Reference") (OtherComp :type "PrimitiveComponent Object Reference") (NormalImpulse :type "Vector Structure") (Hit :type "HitResult Structure (by ref)"))
  (if (== (`GameplayStatics.GetObjectClass` OtherActor) "/Game/LevelPrototyping/Blueprints/BP_TopDownCharacter.BP_TopDownCharacter_C")
    (bind _asbp_top_down_character (cast `/Game/LevelPrototyping/Blueprints/BP_TopDownCharacter` OtherActor))
    (if (`self.pigDashNeeded`)
      (if (`|EnumEquality` (`/Game/LevelPrototyping/Blueprints/BP_TopDownCharacter.pigMoveState` _asbp_top_down_character) "NewEnumerator2")
        (`|ExecutionSequence` :!label _label
          (:`then_0`
            (if (`self.isBouncy`)
              (`self.bounceEvent` _asbp_top_down_character)
              (`SceneComponent.SetWorldScale3D` (`self.Cube`) (1.0 1.0 1.0))
              (bind (_direction _newtrack_0) (`Timeline|bounceGrow` :!via `PlayFromStart`)
                (:`Update`
                  (`SceneComponent.SetWorldScale3D` (`self.Cube`) (`KismetMathLibrary.MakeVector` _newtrack_0 _newtrack_0 _newtrack_0))))))
          (:`then_1`
            (if (`self.isDestructable`)
              (if (not (`self.isFragile`))
                (set `self.isBeingDestroyed` true)
                (`PrimitiveComponent.SetEnableGravity` (`self.Cube`) true)
                (`KismetSystemLibrary.Delay` 5.0)
                (bind (_direction_2 _shrinkdespawntrack) (`Timeline|Timeline_0`)
                  (:`Update`
                    (`SceneComponent.SetWorldScale3D` (`self.Cube`) (`KismetMathLibrary.MakeVector` _shrinkdespawntrack _shrinkdespawntrack _shrinkdespawntrack)))
                  (:`Finished`
                    (`self.K2_DestroyActor`))))))))
      (else
        (goto _label)))))

(fn `bounceEvent`
  (params (player :type "/Game/LevelPrototyping/Blueprints/BP_TopDownCharacter Object Reference"))
  (`Character.LaunchCharacter` player (* (`KismetMathLibrary.GetDirectionUnitVector` (`self.K2_GetActorLocation`) (`self.K2_GetActorLocation` player)) (`self.bounceStrength`)) true true))

(fn `UserConstructionScript`)