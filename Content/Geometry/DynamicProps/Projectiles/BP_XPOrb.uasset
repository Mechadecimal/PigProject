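; BP_XPOrb is an experience pickup projectile that flies to the pig character and grants it XP.
; It launches at a start velocity; when the pig enters PickupRange, it gets pushed away from the pig and homes on its capsule.
; After a short delay, a timeline lerps it onto the pig's position.
; Overlapping SphereRange with the pig adds XP, plays a munching sound and destroys the orb.
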(event `self.ReceiveBeginPlay`
  (set `MovementComponent.Velocity` (`self.startVelocity`) (`self.ProjectileMovement`)))

(event `self.PickupRange.OnComponentBeginOverlap`
  (params (OverlappedComponent :type "PrimitiveComponent Object Reference") (OtherActor :type "Actor Object Reference") (OtherComp :type "PrimitiveComponent Object Reference") (OtherBodyIndex :type Integer) (bFromSweep :type Boolean) (SweepResult :type "HitResult Structure (by ref)"))
  (if (== (`GameplayStatics.GetObjectClass` OtherActor) "/Game/LevelPrototyping/Blueprints/BP_Pig.BP_Pig_C")
    (if (not (`self.isFlying`))
      (bind _asbp_pig (cast `/Game/LevelPrototyping/Blueprints/BP_Pig` OtherActor))
      (`self.FlyToPig` _asbp_pig)
      (`GameplayStatics.PlaySound2D` "/Game/Sounds/XpMovingToPlayer.XpMovingToPlayer" 1.0 1.0 0.0 null null)
      (`KismetSystemLibrary.Delay` 0.5)
      (bind (_direction _newtrack_0) (`Timeline|Timeline_0` :!via `PlayFromStart`)
        (:`Update`
          (`self.K2_SetActorLocation` (`KismetMathLibrary.VLerp` (`self.K2_GetActorLocation`) (`self.K2_GetActorLocation` _asbp_pig) _newtrack_0) true))))))

(event `self.SphereRange.OnComponentBeginOverlap`
  (params (OverlappedComponent :type "PrimitiveComponent Object Reference") (OtherActor :type "Actor Object Reference") (OtherComp :type "PrimitiveComponent Object Reference") (OtherBodyIndex :type Integer) (bFromSweep :type Boolean) (SweepResult :type "HitResult Structure (by ref)"))
  (if (== (`GameplayStatics.GetObjectClass` OtherActor) "/Game/LevelPrototyping/Blueprints/BP_Pig.BP_Pig_C")
    (bind _asbp_pig (cast `/Game/LevelPrototyping/Blueprints/BP_Pig` OtherActor))
    (`/Game/LevelPrototyping/Blueprints/BP_Pig.AddXP` _asbp_pig 1)
    (`GameplayStatics.PlaySound2D` "/Game/Sounds/CornMunchin.CornMunchin" 1.0 1.0 0.25 null null)
    (set `self.isFlying` true)
    (`self.K2_DestroyActor`)))

(event `FlyToPig`
  (params (Pig :type "/Game/LevelPrototyping/Blueprints/BP_Pig Object Reference"))
  (bind _projectilemovement (`self.ProjectileMovement`))
  (set `ProjectileMovementComponent.HomingTargetComponent` (`Character.CapsuleComponent` Pig) _projectilemovement)
  (set `MovementComponent.Velocity` (+ (`MovementComponent.Velocity` _projectilemovement) (* (`KismetMathLibrary.GetDirectionUnitVector` (`self.K2_GetActorLocation` Pig) (`self.K2_GetActorLocation`)) 500)) _projectilemovement)
  (set `self.isFlying` true))

(fn `UserConstructionScript`)