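; BP_XPOrbPickup is an experience orb pickup that grants XP to the pig character when touched.
; Pickup only becomes possible half a second after spawn, via a delayed CanPickup flag.
; On SphereRange overlap, an exact class check for BP_Pig gates a call to AddXP with the orb's XP amount, after which the orb destroys itself.
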(event `self.ReceiveBeginPlay`
  (`KismetSystemLibrary.Delay` 0.5)
  (set `self.canPickup` true))

(event `self.SphereRange.OnComponentBeginOverlap`
  (params (OverlappedComponent :type "PrimitiveComponent Object Reference") (OtherActor :type "Actor Object Reference") (OtherComp :type "PrimitiveComponent Object Reference") (OtherBodyIndex :type Integer) (bFromSweep :type Boolean) (SweepResult :type "HitResult Structure (by ref)"))
  (if (`self.canPickup`)
    (if (== (`GameplayStatics.GetObjectClass` OtherActor) "/Game/LevelPrototyping/Blueprints/BP_Pig.BP_Pig_C")
      (bind _asbp_pig (cast `/Game/LevelPrototyping/Blueprints/BP_Pig` OtherActor))
      (`/Game/LevelPrototyping/Blueprints/BP_Pig.AddXP` _asbp_pig (`self.xpAmmount`))
      (`self.K2_DestroyActor`))))

(fn `UserConstructionScript`)