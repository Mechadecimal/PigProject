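; Base level prop that reacts to hits from BP_Pig, optionally gated on the pig's move state through PigDashNeeded.
; InteractFunc launches the pig away with a scale animation if bouncy, and awards game mode points if destructible.
; Destructibles either call BecomeShatter, a sound-only stub for children, or turn physical, then shrink and despawn after a delay.
; Non-pig hits also turn destructibles physical, without points.
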(event `Bounce`
  (params (pig :type "/Game/LevelPrototyping/Blueprints/BP_Pig Object Reference"))
  (`self.bounceEvent` pig)
  (`SceneComponent.SetWorldScale3D` (`self.Cube`) (1.0 1.0 1.0))
  (`GameplayStatics.PlaySoundAtLocation` "/Game/Sounds/Pinball.Pinball" (`self.K2_GetActorLocation`) (struct) 1.0 1.0 0.0 null null null null)
  (bind (_direction _newtrack_0) (`Timeline|Timeline_1` :!via `PlayFromStart`)
    (:`Update`
      (`SceneComponent.SetWorldScale3D` (`self.Cube`) (`KismetMathLibrary.MakeVector` _newtrack_0 _newtrack_0 _newtrack_0)))))

(event `DestroySequence`
  (set `self.isBeingDestroyed` true)
  (`KismetSystemLibrary.Delay` 5.0)
  (bind (_direction _shrinkdespawntrack) (`Timeline|Timeline_0`)
    (:`Update`
      (`SceneComponent.SetWorldScale3D` (`self.Cube`) (`KismetMathLibrary.MakeVector` _shrinkdespawntrack _shrinkdespawntrack _shrinkdespawntrack)))
    (:`Finished`
      (`self.K2_DestroyActor`))))

(event `self.Cube.OnComponentHit`
  (params (HitComponent :type "PrimitiveComponent Object Reference") (OtherActor :type "Actor Object Reference") (OtherComp :type "PrimitiveComponent Object Reference") (NormalImpulse :type "Vector Structure") (Hit :type "HitResult Structure (by ref)"))
  (if (== (`GameplayStatics.GetObjectClass` OtherActor) "/Game/LevelPrototyping/Blueprints/BP_Pig.BP_Pig_C")
    (bind _asbp_pig (cast `/Game/LevelPrototyping/Blueprints/BP_Pig` OtherActor))
    (if (`self.pigDashNeeded`)
      (if (`|EnumEquality` (`/Game/LevelPrototyping/Blueprints/BP_Pig.pigMoveState` _asbp_pig) "NewEnumerator2")
        (`self.interactFunc` _asbp_pig :!label _label))
      (else
        (goto _label)))
    (else
      (`GameplayStatics.PlaySoundAtLocation` "/Game/Sounds/Flap.Flap" (`self.K2_GetActorLocation`) (struct) 1.0 1.0 0.0 null null null null)
      (if (`self.isDestructable`)
        (if (not (`self.isBeingDestroyed`))
          (`self.becomeDynamic`))))))

(fn `becomeDynamic`
  (bind _cube (`self.Cube`))
  (`GameplayStatics.PlaySoundAtLocation` null (`self.K2_GetActorLocation`) (struct) 1.0 1.0 0.0 null null null null)
  (`PrimitiveComponent.WakeAllRigidBodies` _cube)
  (`PrimitiveComponent.SetCollisionEnabled` _cube "QueryAndPhysics")
  (`PrimitiveComponent.SetSimulatePhysics` _cube true)
  (`self.DestroySequence`))

(fn `becomeShatter`
  ;[1 1 1] should be implemented by children
  (`GameplayStatics.PlaySoundAtLocation` "/Game/Sounds/metalCrate.metalCrate" (`self.K2_GetActorLocation`) (struct) 1.0 1.0 0.0 null null null null))

(fn `bounceEvent`
  (params (player :type "/Game/LevelPrototyping/Blueprints/BP_Pig Object Reference"))
  (`Character.LaunchCharacter` player (* (`KismetMathLibrary.GetDirectionUnitVector` (`self.K2_GetActorLocation`) (`self.K2_GetActorLocation` player)) (`self.bounceStrength`)) true true))

(fn `interactFunc`
  (params (Pig :type "/Game/LevelPrototyping/Blueprints/BP_Pig Object Reference"))
  (if (not (`self.isBeingDestroyed`))
    (`|ExecutionSequence`
      (:`then_0`
        (if (`self.isBouncy`)
          (`self.Bounce` Pig)))
      (:`then_1`
        (if (`self.isDestructable`)
          (bind _asbp_top_down_game_mode (cast `/Game/LevelPrototyping/Blueprints/BP_TopDownGameMode` (`GameplayStatics.GetGameMode`)))
          (`/Game/LevelPrototyping/Blueprints/BP_TopDownGameMode.AddPoints` _asbp_top_down_game_mode (`self.DestructionPoints`))
          (if (`self.isFragile`)
            (`self.becomeShatter`)
            (else
              (`self.becomeDynamic`))))))))

(fn `UserConstructionScript`)