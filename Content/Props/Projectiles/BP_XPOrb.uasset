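; XP orb pickup that flies to the top-down player character and grants experience.
; Entering PickupRange calls FlyToPig once, which kicks the orb away from the player and sets the player's capsule as the ProjectileMovement homing target.
; After a short delay, a timeline lerps the orb's location toward the player's current position with sweep.
; Overlapping SphereRange with the player adds one XP and destroys the orb.
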(event `self.PickupRange.OnComponentBeginOverlap`
  (params (OverlappedComponent :type "PrimitiveComponent Object Reference") (OtherActor :type "Actor Object Reference") (OtherComp :type "PrimitiveComponent Object Reference") (OtherBodyIndex :type Integer) (bFromSweep :type Boolean) (SweepResult :type "HitResult Structure (by ref)"))
  (if (== (`GameplayStatics.GetObjectClass` OtherActor) "/Game/TopDown/Blueprints/BP_TopDownCharacter.BP_TopDownCharacter_C")
    (if (not (`self.isFlying`))
      (bind _asbp_top_down_character (cast `/Game/TopDown/Blueprints/BP_TopDownCharacter` OtherActor))
      (`self.FlyToPig` _asbp_top_down_character)
      (`KismetSystemLibrary.Delay` 0.5)
      (bind (_direction _newtrack_0) (`Timeline|Timeline_0` :!via `PlayFromStart`)
        (:`Update`
          (`self.K2_SetActorLocation` (`KismetMathLibrary.VLerp` (`self.K2_GetActorLocation`) (`self.K2_GetActorLocation` _asbp_top_down_character) _newtrack_0) true))))))

(event `self.SphereRange.OnComponentBeginOverlap`
  (params (OverlappedComponent :type "PrimitiveComponent Object Reference") (OtherActor :type "Actor Object Reference") (OtherComp :type "PrimitiveComponent Object Reference") (OtherBodyIndex :type Integer) (bFromSweep :type Boolean) (SweepResult :type "HitResult Structure (by ref)"))
  (if (== (`GameplayStatics.GetObjectClass` OtherActor) "/Game/TopDown/Blueprints/BP_TopDownCharacter.BP_TopDownCharacter_C")
    (bind _asbp_top_down_character (cast `/Game/TopDown/Blueprints/BP_TopDownCharacter` OtherActor))
    (`/Game/TopDown/Blueprints/BP_TopDownCharacter.AddXP` _asbp_top_down_character 1)
    (`self.K2_DestroyActor`)))

(event `FlyToPig`
  (params (Pig :type "/Game/TopDown/Blueprints/BP_TopDownCharacter Object Reference"))
  (bind _projectilemovement (`self.ProjectileMovement`))
  (set `ProjectileMovementComponent.HomingTargetComponent` (`Character.CapsuleComponent` Pig) _projectilemovement)
  (set `MovementComponent.Velocity` (+ (`MovementComponent.Velocity` _projectilemovement) (* (`KismetMathLibrary.GetDirectionUnitVector` (`self.K2_GetActorLocation` Pig) (`self.K2_GetActorLocation`)) 500)) _projectilemovement)
  (set `self.isFlying` true))

(fn `UserConstructionScript`)