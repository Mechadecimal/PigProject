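; Shatterable prop Blueprint that drops XP orbs when it breaks.
; It extends the parent's BecomeShatter by spawning BP_XPOrb actors according to XPDrop, then destroying itself.
; SpawnXP launches each orb from the prop's location with a randomized projectile velocity, clamping the vertical component so orbs never start moving downward.
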(fn `becomeShatter`
  (`parent.becomeShatter`)
  (`self.SpawnXP` (`self.XPDrop`))
  (`self.K2_DestroyActor`))

(fn `SpawnXP`
  (params (xp :type Integer))
  (for _ (range (+ xp 1))
    (bind _returnvalue (`|SpawnActorFromClass` "/Game/Props/Projectiles/BP_XPOrb.BP_XPOrb_C" (`KismetMathLibrary.MakeTransform` (`self.K2_GetActorLocation`)) "Undefined" "OverrideRootScale" null null))
    (set `MovementComponent.Velocity` (`KismetMathLibrary.MakeVector` (.x (* (`KismetMathLibrary.RandomUnitVector`) 1000)) (.y (* (`KismetMathLibrary.RandomUnitVector`) 1000)) (`KismetMathLibrary.FMax` (.z (* (`KismetMathLibrary.RandomUnitVector`) 1000)))) (`/Game/Props/Projectiles/BP_XPOrb.ProjectileMovement` _returnvalue))))

(fn `UserConstructionScript`
  (`parent.UserConstructionScript`))