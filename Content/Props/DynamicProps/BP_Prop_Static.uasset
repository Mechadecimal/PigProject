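; BP_Prop_Static is a prop that can bounce the top-down character away when it hits the Cube component.
; PigDashNeeded optionally restricts the reaction to one specific PigMoveState, presumably the dash, and IsBouncy enables the launch.
; The launch overrides XY and Z velocity with the prop-to-character direction scaled by BounceStrength, plus the character's world location, so the result varies with map position.
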(event `self.Cube.OnComponentHit`
  (params (HitComponent :type "PrimitiveComponent Object Reference") (OtherActor :type "Actor Object Reference") (OtherComp :type "PrimitiveComponent Object Reference") (NormalImpulse :type "Vector Structure") (Hit :type "HitResult Structure (by ref)"))
  (if (== (`GameplayStatics.GetObjectClass` OtherActor) "/Game/TopDown/Blueprints/BP_TopDownCharacter.BP_TopDownCharacter_C")
    (bind _asbp_top_down_character (cast `/Game/TopDown/Blueprints/BP_TopDownCharacter` OtherActor))
    (if (`self.pigDashNeeded`)
      (if (`|EnumEquality` (`/Game/TopDown/Blueprints/BP_TopDownCharacter.pigMoveState` _asbp_top_down_character) "NewEnumerator2")
        (`|ExecutionSequence` :!label _label
          (:`then_0`
            (if (`self.isBouncy`)
              (bind _returnvalue (`self.K2_GetActorLocation` _asbp_top_down_character))
              (`Character.LaunchCharacter` _asbp_top_down_character (+ (* (`KismetMathLibrary.GetDirectionUnitVector` (`self.K2_GetActorLocation`) _returnvalue) (`self.bounceStrength`)) _returnvalue) true true)))))
      (else
        (goto _label)))))

(fn `UserConstructionScript`)